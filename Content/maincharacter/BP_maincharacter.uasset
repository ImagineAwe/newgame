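; Player character Blueprint with Enhanced Input movement, sprint, aiming and shooting.
; BeginPlay attaches a spawned BP_weapon1, adds the mapping context and shows the crosshair HUD.
; Aiming hides the HUD and slides the camera by timeline; aiming and shooting lock yaw to the controller.
; DoOnce plus Delay throttles fire, which decrements ammo, plays sounds and traces from camera, then muzzle to that target, with debug lines but no damage.
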(event `EnhancedInput|/Game/data/inputs/IA_move`
  (params (ActionValue :type "Vector2D Structure") (ElapsedSeconds :type "Float (double-precision)") (TriggeredSeconds :type "Float (double-precision)") (InputAction :type "InputAction Object Reference" :default "/Game/data/inputs/IA_move.IA_move"))
  (bind (_returnvalue_roll _returnvalue_pitch _returnvalue_yaw) (`KismetMathLibrary.BreakRotator` (`self.GetControlRotation`)))
  (bind (_returnvalue_roll_2 _returnvalue_pitch_2 _returnvalue_yaw_2) (`KismetMathLibrary.BreakRotator` (`self.GetControlRotation`)))
  ; движение персонажа
  (:`Triggered`
    ;; движение влево (вправо)
    (`self.AddMovementInput` (`KismetMathLibrary.GetRightVector` (`KismetMathLibrary.MakeRotator` _returnvalue_roll 0.0 _returnvalue_yaw)) ActionValue_X)
    ;; движение вперед (назад)
    (`self.AddMovementInput` (`KismetMathLibrary.GetForwardVector` (`KismetMathLibrary.MakeRotator` 0.0 0.0 _returnvalue_yaw_2)) ActionValue_Y)))

(event `self.ReceiveBeginPlay`
  (`|ExecutionSequence`
    (:`then_0`
      ; оружие
      (bind _returnvalue (`|SpawnActorFromClass` "/Game/FPS_Weapon_Bundle/BP_weapon1.BP_weapon1_C" (`SceneComponent.GetSocketTransform` (`self.Mesh`) "weapon1socket" "RTS_World") "Undefined" "MultiplyWithRoot" null null))
      (bind _output_get (set `self.BP_weapon1` _returnvalue))
      (`self.K2_AttachToComponent` _output_get (`self.Mesh`) "weapon1socket" "SnapToTarget" "SnapToTarget" "SnapToTarget" true))
    (:`then_1`
      ; подключение кнопок
      (bind _asplayer_controller (cast `PlayerController` (`self.GetController`)))
      (`EnhancedInputSubsystemInterface.AddMappingContext` (pcsubsystem `EnhancedInputLocalPlayerSubsystem` _asplayer_controller) "/Game/data/inputs/IMC_default.IMC_default" 0 (struct)))
    (:`then_2`
      ; прицел
      (bind _returnvalue_2 (`|CreateWidget` "/Game/data/widgets/WBP_HUD.WBP_HUD_C"))
      (bind _output_get_2 (set `self.WBP_HUD` _returnvalue_2))
      (`UserWidget.AddToViewport` _output_get_2 0))))

(event `EnhancedInput|/Game/data/inputs/IA_look`
  (params (ActionValue :type "Vector2D Structure") (ElapsedSeconds :type "Float (double-precision)") (TriggeredSeconds :type "Float (double-precision)") (InputAction :type "InputAction Object Reference" :default "/Game/data/inputs/IA_look.IA_look"))
  ; камера
  (:`Triggered`
    ;; камера лево/право
    (`self.AddControllerYawInput` ActionValue_X)
    ;; камера вверх/вниз
    (`self.AddControllerPitchInput` ActionValue_Y)))

(event `EnhancedInput|/Game/data/inputs/IA_shoot`
  (params (ActionValue :type Boolean) (ElapsedSeconds :type "Float (double-precision)") (TriggeredSeconds :type "Float (double-precision)") (InputAction :type "InputAction Object Reference" :default "/Game/data/inputs/IA_shoot.IA_shoot"))
  (:`Triggered`
    (`/Engine/EditorBlueprintResources/StandardMacros.DoOnce` false :!label _label
      (:`Completed`
        (`self.AmmoCounter`)
        (if (`self.bCanShoot`)
          (`/Game/FPS_Weapon_Bundle/BP_weapon1.SpawnLight` (`self.BP_weapon1`))
          (`GameplayStatics.SpawnSound2D` "/Game/data/sounds/shot.shot" 1.0 (`KismetMathLibrary.FClamp` (`KismetMathLibrary.RandomFloat`) 0.9 1.1) 0.0 null)
          (`self.LineTrace`)
          (else
            (`GameplayStatics.SpawnSound2D` "/Game/data/sounds/empty.empty" 1.0 (`KismetMathLibrary.FClamp` (`KismetMathLibrary.RandomFloat`) 0.9 1.1) 0.0 null)))
        (`KismetSystemLibrary.Delay` 0.1)
        (goto _label :!via `Reset`))))
  (:`Completed`
    (set `self.bCanShoot` false)))

(event `EnhancedInput|/Game/data/inputs/IA_sprint`
  (params (ActionValue :type Boolean) (ElapsedSeconds :type "Float (double-precision)") (TriggeredSeconds :type "Float (double-precision)") (InputAction :type "InputAction Object Reference" :default "/Game/data/inputs/IA_sprint.IA_sprint"))
  (bind _charactermovement (`self.CharacterMovement`))
  ; sprint/walking
  (:`Triggered`
    (set `CharacterMovementComponent.MaxWalkSpeed` 400.0 _charactermovement))
  (:`Canceled`
    (set `CharacterMovementComponent.MaxWalkSpeed` 200.0 _charactermovement :!label _label_2))
  (:`Completed`
    (goto _label_2)))

(event `self.ReceiveTick`
  (params (DeltaSeconds :type "Float (single-precision)"))
  (if (== (`self.Ammo`) 0)
    (set `self.bCanShoot` false)
    (else
      (set `self.bCanShoot` true))))

(event `EnhancedInput|/Game/data/inputs/IA_aiming`
  (params (ActionValue :type Boolean) (ElapsedSeconds :type "Float (double-precision)") (TriggeredSeconds :type "Float (double-precision)") (InputAction :type "InputAction Object Reference" :default "/Game/data/inputs/IA_aiming.IA_aiming"))
  (bind _wbp_hud (`self.WBP_HUD`))
  (bind _camera (`self.Camera`))
  (bind (_relativelocation_x _relativelocation_y _relativelocation_z) (`KismetMathLibrary.BreakVector` (`SceneComponent.RelativeLocation` _camera)))
  ; прицел
  (:`Triggered`
    (set `self.bIsAiming` true)
    (set `self.bUseControllerRotationYaw` true)
    ;; при прицеливании удаляет прицел
    (`Widget.RemoveFromParent` _wbp_hud)
    ;; приближение камеры при прицеливании
    (bind (_direction _zoom) (`Timeline|TL_aim` :!label _label_3)
      (:`Update`
        (`SceneComponent.K2_SetRelativeLocation` _camera (`KismetMathLibrary.MakeVector` (`KismetMathLibrary.Lerp` 95.0 160.0 _zoom) _relativelocation_y _relativelocation_z) false false))))
  (:`Canceled`
    (set `self.bIsAiming` false :!label _label_4)
    (set `self.bUseControllerRotationYaw` false)
    ;; добавляет прицел когда отпускаешь пкм
    (`UserWidget.AddToViewport` _wbp_hud 0)
    (goto _label_3 :!via `Reverse`))
  (:`Completed`
    (goto _label_4)))

(event `EnhancedInput|/Game/data/inputs/IA_shoot`
  (params (ActionValue :type Boolean) (ElapsedSeconds :type "Float (double-precision)") (TriggeredSeconds :type "Float (double-precision)") (InputAction :type "InputAction Object Reference" :default "/Game/data/inputs/IA_shoot.IA_shoot"))
  ; поворачивает модельку в сторону стрельбы
  (:`Triggered`
    (set `self.bIsShooting` true)
    (set `self.bUseControllerRotationYaw` true))
  (:`Canceled`
    (set `self.bIsShooting` false :!label _label_5)
    (set `self.bUseControllerRotationYaw` false))
  (:`Completed`
    (goto _label_5)))

(fn `AmmoCounter`
  (bind _output_get (set `self.Ammo` (`KismetMathLibrary.Clamp` (- (`self.Ammo`) 1) 0 30)))
  (`KismetSystemLibrary.PrintString` (`KismetStringLibrary.Conv_IntToString` _output_get)))

(fn `LineTrace`
  (bind _returnvalue (`GameplayStatics.GetPlayerCameraManager` 0))
  (bind _returnvalue_2 (`self.K2_GetActorLocation` _returnvalue))
  (bind _outhit (`KismetSystemLibrary.LineTraceSingle` _returnvalue_2 (+ _returnvalue_2 (* (`self.GetActorForwardVector` _returnvalue) 50000.0)) "TraceTypeQuery1"))
  (bind (_bblockinghit _binitialoverlap _time _distance _location _impactpoint _normal _impactnormal _physmat _hitactor _hitcomponent _hitbonename _bonename _hititem _elementindex _faceindex _tracestart _traceend) (`GameplayStatics.BreakHitResult` _outhit))
  (if _bblockinghit
    (`KismetSystemLibrary.LineTraceSingle` :`Start` (`SceneComponent.K2_GetComponentLocation` (`/Game/FPS_Weapon_Bundle/BP_weapon1.Arrow` (`self.BP_weapon1`))) :`End` _impactpoint :`TraceChannel` "TraceTypeQuery1" :`DrawDebugType` "ForDuration")
    (else
      (`KismetSystemLibrary.LineTraceSingle` :`Start` (`SceneComponent.K2_GetComponentLocation` (`/Game/FPS_Weapon_Bundle/BP_weapon1.Arrow` (`self.BP_weapon1`))) :`End` _traceend :`TraceChannel` "TraceTypeQuery1" :`DrawDebugType` "ForDuration"))))

(fn `UserConstructionScript`)